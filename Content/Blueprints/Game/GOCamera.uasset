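; GOCamera is a camera Blueprint that pans its CineCamera sideways in response to swipe input.
; When a left or right swipe ends on its Swipe component, it shifts the CineCamera's relative location a fixed step along Y, negative for left and positive for right, with sweep enabled.
; Each swipe also prints a debug string, and the move is instant with no interpolation or bounds.
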(event `self.ReceiveBeginPlay`)

(event `self.Swipe.SwipeLeftEnded`
  (params (StartLocation :type "Vector2D Structure") (TriggerLocation :type "Vector2D Structure") (EndLocation :type "Vector2D Structure"))
  (bind _cinecamera (`self.CineCamera`))
  (`KismetSystemLibrary.PrintString` "SwipeLeft")
  (`SceneComponent.K2_SetRelativeLocation` _cinecamera (`KismetMathLibrary.MakeVector` (.x (`SceneComponent.RelativeLocation` _cinecamera)) (- (.y (`SceneComponent.RelativeLocation` _cinecamera)) 300.0) (.z (`SceneComponent.RelativeLocation` _cinecamera))) true false))

(event `self.Swipe.SwipeRightEnded`
  (params (StartLocation :type "Vector2D Structure") (TriggerLocation :type "Vector2D Structure") (EndLocation :type "Vector2D Structure"))
  (bind _cinecamera (`self.CineCamera`))
  (`KismetSystemLibrary.PrintString` "SwipeRight")
  (`SceneComponent.K2_SetRelativeLocation` _cinecamera (`KismetMathLibrary.MakeVector` (.x (`SceneComponent.RelativeLocation` _cinecamera)) (+ (.y (`SceneComponent.RelativeLocation` _cinecamera)) 300.0) (.z (`SceneComponent.RelativeLocation` _cinecamera))) true false))

(fn `UserConstructionScript`)