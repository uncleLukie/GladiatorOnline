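; Game mode that spawns each joining player's selected character at a random free player start.
; On PostLogin, the server records the controller, shuffles the PlayerStarts, reads the character class from GOPlayerState and spawns it at the first start tagged "unused", then retags that start "used".
; ResetPlayers holds validity-checked teleports with opposing rotations, but their targets are unset.
; StartMap, BeginPlay and Tick are empty.
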(event `StartMap`)

(event `ResetPlayers`
  (`/Engine/EditorBlueprintResources/StandardMacros.IsValid` null
    (:`Is Valid`
      (`self.K2_TeleportTo` (`self.K2_GetActorLocation`) (struct :`Yaw` 90.0))
      (`/Engine/EditorBlueprintResources/StandardMacros.IsValid` null
        (:`Is Valid`
          (`self.K2_TeleportTo` (`self.K2_GetActorLocation`) (struct :`Yaw` 270.0)))))))

(event `self.ReceiveBeginPlay`)

(event `self.K2_PostLogin`
  (params (NewPlayer :type "PlayerController Object Reference"))
  (bind _selectedcharacterplayerstate (`/Game/Blueprints/Game/GOPlayerState.SelectedCharacterPlayerState` (`self.PlayerStateRef`)))
  (`/Engine/EditorBlueprintResources/ActorMacros.Switch Has Authority`
    (:`Authority`
      (bind _asgoplayer_controller (cast `/Game/Blueprints/Game/GOPlayerController` NewPlayer))
      (`KismetArrayLibrary.Array_Add` (`self.PlayerControllerArray`) _asgoplayer_controller)
      (bind _outactors (`GameplayStatics.GetAllActorsOfClass` "/Script/Engine.PlayerStart"))
      (bind _output_get (set `self.PlayerStartArray` _outactors))
      (`KismetArrayLibrary.Array_Shuffle` _output_get)
      (bind _asgoplayer_state (cast `/Game/Blueprints/Game/GOPlayerState` (`Controller.PlayerState` _asgoplayer_controller)))
      (set `self.PlayerStateRef` _asgoplayer_state)
      (`KismetSystemLibrary.PrintString` (`KismetSystemLibrary.GetClassDisplayName` _selectedcharacterplayerstate))
      (for _array_element (`self.PlayerStartArray`)
        (if (== (`PlayerStart.PlayerStartTag` _array_element) "unused")
          (`|SpawnActorFromClass` _selectedcharacterplayerstate (`self.GetTransform` _array_element) "AlwaysSpawn" "OverrideRootScale" NewPlayer null)
          (set `PlayerStart.PlayerStartTag` "used" _array_element)
          (break))))))

(fn `UserConstructionScript`)