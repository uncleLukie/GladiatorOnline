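; Game instance for GladiatorOnline that opens the UI screens: loading, login, main menu, register and profile.
; Each show event creates its widget for player controller 0 when the cached reference is invalid, stores it, then adds a widget to the viewport.
; ShowLoadingScreen caches the loading widget but adds the login widget reference to the viewport instead.
; No event here removes a screen that is already shown.
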(event `ShowLoadingScreen`
  ;[1 1 1] Show loading screen
  (`/Engine/EditorBlueprintResources/StandardMacros.IsValid` (`self.LoadingScreenWidgetRef`)
    (:`Is Valid`
      _)
    (:`Is Not Valid`
      (bind _returnvalue (`|CreateWidget` "/Game/GladiatorOnline/Blueprints/UI/LoadingScreen.LoadingScreen_C" (`GameplayStatics.GetPlayerController` 0)))
      (set `self.LoadingScreenWidgetRef` _returnvalue)))
  (`UserWidget.AddToViewport` (`self.LoginScreenWidgetRef`) 0))

(event `Show Login Screen`
  ;[1 1 1] Show login screen
  (`/Engine/EditorBlueprintResources/StandardMacros.IsValid` (`self.LoginScreenWidgetRef`)
    (:`Is Valid`
      _)
    (:`Is Not Valid`
      (bind _returnvalue (`|CreateWidget` "/Game/GladiatorOnline/Blueprints/UI/LoginScreen.LoginScreen_C" (`GameplayStatics.GetPlayerController` 0)))
      (set `self.LoginScreenWidgetRef` _returnvalue)))
  (`UserWidget.AddToViewport` (`self.LoginScreenWidgetRef`) 0))

(event `Show Main Menu`
  ;[1 1 1] Show main menu
  (`/Engine/EditorBlueprintResources/StandardMacros.IsValid` (`self.MainMenuWidgetRef`)
    (:`Is Valid`
      _)
    (:`Is Not Valid`
      (bind _returnvalue (`|CreateWidget` "/Game/GladiatorOnline/Blueprints/UI/MainMenuScreen.MainMenuScreen_C" (`GameplayStatics.GetPlayerController` 0)))
      (set `self.MainMenuWidgetRef` _returnvalue)))
  (`UserWidget.AddToViewport` (`self.MainMenuWidgetRef`) 0))

(event `Show Register Screen`
  ;[1 1 1] Show Register Screen
  (`/Engine/EditorBlueprintResources/StandardMacros.IsValid` (`self.RegisterScreenWidgetRef`)
    (:`Is Valid`
      _)
    (:`Is Not Valid`
      (bind _returnvalue (`|CreateWidget` "/Game/GladiatorOnline/Blueprints/UI/RegisterScreen.RegisterScreen_C" (`GameplayStatics.GetPlayerController` 0)))
      (set `self.RegisterScreenWidgetRef` _returnvalue)))
  (`UserWidget.AddToViewport` (`self.RegisterScreenWidgetRef`) 0))

(event `ShowProfileScreen`
  ;[1 1 1] Show Profile Screen
  (`/Engine/EditorBlueprintResources/StandardMacros.IsValid` (`self.ProfileWidgetRef`)
    (:`Is Valid`
      _)
    (:`Is Not Valid`
      (bind _returnvalue (`|CreateWidget` "/Game/GladiatorOnline/Blueprints/UI/ProfileScreen.ProfileScreen_C" (`GameplayStatics.GetPlayerController` 0)))
      (set `self.ProfileWidgetRef` _returnvalue)))
  (`UserWidget.AddToViewport` (`self.ProfileWidgetRef`) 0))